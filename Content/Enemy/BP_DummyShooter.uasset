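; BP_DummyShooter is an enemy character that takes damage, dies, and detects pawns by sight.
; AnyDamage passes through a DoOnce with no visible reset, so only the first hit reduces Health.
; At zero or below it plays a fall montage, waits briefly, then destroys itself.
; PawnSensing sets IsSeeingPlayer on any sighting and prints a debug message; no shooting logic is present.
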(event `self.ReceiveAnyDamage`
  (params (Damage :type "Float (single-precision)") (DamageType :type "DamageType Object Reference") (InstigatedBy :type "Controller Object Reference") (DamageCauser :type "Actor Object Reference"))
  ;[1 1 1] Recieve damage
  (`/Engine/EditorBlueprintResources/StandardMacros.DoOnce` false
    (:`Completed`
      (bind _output_get (set `self.Health` (`KismetMathLibrary.FTrunc` (- (`self.Health`) Damage))))
      (if (<= _output_get 0)
        (`self.PlayAnimMontage` "/Game/Characters/Mannequins/Animations/Manny/MM_Fall_Loop_Montage.MM_Fall_Loop_Montage")
        (`KismetSystemLibrary.Delay` 0.1)
        (`self.K2_DestroyActor`)))))

(event `self.PawnSensing.OnSeePawn`
  (params (Pawn :type "Pawn Object Reference"))
  (set `self.IsSeeingPlayer` true)
  (`KismetSystemLibrary.PrintString` "Is seeing player"))

(fn `UserConstructionScript`)