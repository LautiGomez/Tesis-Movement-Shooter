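; BP_Grapple_Hook is the projectile actor for the player's grapple hook.
; On BeginPlay it copies its Velocity variable into the ProjectileMovement component and records its spawn location.
; Each Tick it measures straight-line distance from that start point and destroys itself on reaching MaxRange.
; It contains no hit, attach or pull logic.
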(event `self.ReceiveBeginPlay`
  (set `MovementComponent.Velocity` (`self.Velocity`) (`self.ProjectileMovement`))
  (set `self.Start Location` (`self.K2_GetActorLocation`)))

(event `self.ReceiveTick`
  (params (DeltaSeconds :type "Float (single-precision)"))
  (if (>= (`KismetMathLibrary.Vector_Distance` (`self.Start Location`) (`self.K2_GetActorLocation`)) (`self.Max Range`))
    (`self.K2_DestroyActor`)))

(fn `UserConstructionScript`)