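; Fire hazard actor that deals repeated damage to the player while they stay inside its collision sphere.
; On BeginPlay it plays a sound at its location and caches player 0 as a BP_FirstPersonCharacter.
; An overlap by a Player-tagged actor starts a looping half-second timer that applies damage to that cached character.
; Ending the overlap clears the timer.
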(event `self.ReceiveBeginPlay`
  (`|ExecutionSequence`
    (:`then_0`
      (`GameplayStatics.PlaySoundAtLocation` null (`self.K2_GetActorLocation`) (struct) 1.0 1.0 0.0 null null null null))
    (:`then_1`
      (bind _asbp_first_person_character (cast `/Game/Player/Blueprints/BP_FirstPersonCharacter` (`GameplayStatics.GetPlayerCharacter` 0)))
      (set `self.BP First Person Character` _asbp_first_person_character))))

(event `self.Sphere Collision.OnComponentBeginOverlap`
  (params (OverlappedComponent :type "PrimitiveComponent Object Reference") (OtherActor :type "Actor Object Reference") (OtherComp :type "PrimitiveComponent Object Reference") (OtherBodyIndex :type Integer) (bFromSweep :type Boolean) (SweepResult :type "HitResult Structure (by ref)"))
  (if (`self.ActorHasTag` OtherActor "Player")
    (bind _returnvalue (`KismetSystemLibrary.K2_SetTimerDelegate` (delegate `Damage`) 0.5 true))
    (set `self.REF Timer Damage` _returnvalue)))

(event `Damage`
  (`GameplayStatics.ApplyDamage` (`self.BP First Person Character`) 5.0 null self))

(event `self.Sphere Collision.OnComponentEndOverlap`
  (params (OverlappedComponent :type "PrimitiveComponent Object Reference") (OtherActor :type "Actor Object Reference") (OtherComp :type "PrimitiveComponent Object Reference") (OtherBodyIndex :type Integer))
  (if (`self.ActorHasTag` OtherActor "Player")
    (`KismetSystemLibrary.K2_ClearAndInvalidateTimerHandle` (`self.REF Timer Damage`))))

(fn `UserConstructionScript`)